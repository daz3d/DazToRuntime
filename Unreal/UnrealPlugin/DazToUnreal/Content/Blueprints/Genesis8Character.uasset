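; Genesis 8 character Blueprint with modular body and clothing meshes, set up for Live Link ARKit face capture.
; On BeginPlay, a validity-checked macro slaves the head, hair, eyelash, clothing and shoe components to the main Mesh via Master Pose.
; It then casts the anim instance to Genesis81ArkitExample and copies in the actor's Live Link subject, head rotation, delay, mouth offset and calibration settings.
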(event `self.ReceiveBeginPlay`
  (for _array_element (`|MakeArray` (`self.Shoes`) (`self.FacialHair`) (`self.Eyelashes`) (`self.Head`) (`self.Top`) (`self.Bottoms`))
    (`self.MyMasterPoseComponent` _array_element (`self.Mesh`)))
  (bind _asgenesis_81arkit_example (cast `/DazToUnreal/Genesis8_1/Animation/Genesis81ArkitExample` (`SkeletalMeshComponent.GetAnimInstance` (`self.Mesh`))))
  (set `/DazToUnreal/Genesis8_1/Animation/Genesis81ArkitExample.LiveLinkSubject` (`self.LiveLinkSubject`) _asgenesis_81arkit_example)
  (set `/DazToUnreal/Genesis8_1/Animation/Genesis81ArkitExample.Using Local Rotations` (`self.UsingLocalRotations`) _asgenesis_81arkit_example)
  (set `/DazToUnreal/Genesis8_1/Animation/Genesis81ArkitExample.HeadRotationStrength` (`self.HeadRotationStrength`) _asgenesis_81arkit_example)
  (set `/DazToUnreal/Genesis8_1/Animation/Genesis81ArkitExample.FaceCaptureDelay` (`self.FaceCaptureDelay`) _asgenesis_81arkit_example)
  (set `/DazToUnreal/Genesis8_1/Animation/Genesis81ArkitExample.MouthOpenOffset` (`self.MouthOpenOffset`) _asgenesis_81arkit_example)
  (set `/DazToUnreal/Genesis8_1/Animation/Genesis81ArkitExample.Calibration` (`self.CalibratedBlendshapes`) _asgenesis_81arkit_example)
  (set `/DazToUnreal/Genesis8_1/Animation/Genesis81ArkitExample.UseCalibration` (`self.AccountCalibration`) _asgenesis_81arkit_example))

(fn `UserConstructionScript`
  (locals (Clothing :type "SkeletalMeshComponent Object Reference" :default null)))