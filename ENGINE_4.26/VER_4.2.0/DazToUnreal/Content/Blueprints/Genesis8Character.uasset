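; Character Blueprint for a Genesis 8 model that hands Live Link settings to its Genesis 8.1 ARKit example animation Blueprint.
; The construction script infers whether the mesh uses local rotations by testing for a zero root socket rotation in component space, then orients the mesh to match.
; On BeginPlay it copies that flag and the Live Link subject into the mesh's anim instance.
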(event `self.ReceiveBeginPlay`
  (bind _asgenesis_81arkit_example (cast `/DazToUnreal/Animation/Genesis81ArkitExample` (`SkeletalMeshComponent.GetAnimInstance` (`self.Mesh`))))
  (set `/DazToUnreal/Animation/Genesis81ArkitExample.LiveLinkSubject` (`self.LiveLinkSubject`) _asgenesis_81arkit_example)
  (set `/DazToUnreal/Animation/Genesis81ArkitExample.Using Local Rotations` (`self.UsingLocalRotations`) _asgenesis_81arkit_example))

(fn `UserConstructionScript`
  ;[1 1 1] Set Model Rotation
  (bind _output_get (set `self.UsingLocalRotations` (== (.rotation (`SceneComponent.GetSocketTransform` (`self.Mesh`) "root" "RTS_Component")) (struct))))
  (if _output_get
    (`SceneComponent.K2_SetRelativeRotation` :`self` (`self.Mesh`))
    (else
      (`SceneComponent.K2_SetRelativeRotation` (`self.Mesh`) (struct :`Yaw` -90.0) false false))))